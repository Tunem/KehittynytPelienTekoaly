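; DoorSparks is an actor with an animated skeletal mesh, apparently a door, and two spark particle systems that emit while it animates.
; Sparks start disabled, and Tick matches both emitters to whether the mesh is playing.
; A looping timer set at BeginPlay calls PlayRateChange, randomizing the animation play rate and each system's spawn-rate parameter for irregular motion and sparking.
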(event EventBeginPlay
  (|CallParentFunction)
  (Utilities|FlowControl|Sequence
    (:then_0
      (Effects|Components|ParticleSystem|SetEmitterEnable (Variables|Default|GetSparksPS) "Sparks" false)
      (Effects|Components|ParticleSystem|SetEmitterEnable (Variables|Default|GetSparksPS1) "Sparks" false))
    (:then_1
      (Utilities|Time|SetTimerbyFunctionName 0 "PlayRateChange" 0.5 true))))

(event Collision|EventActorBeginOverlap
  (params (OtherActor :type Actor%20Object%20Reference))
  (|CallParentFunction OtherActor) ; This node is disabled and will not be called.\nDrag off pins to build functionality.
)

(event EventTick
  (params (DeltaSeconds :type Float%20%28single-precision%29))
  (bind _skeletalmeshcomponent (Variables|Default|GetSkeletalMeshComponent))
  (bind _returnvalue (Audio|Components|Audio|IsPlaying _skeletalmeshcomponent))
  (|CallParentFunction DeltaSeconds)
  (Effects|Components|ParticleSystem|SetEmitterEnable (Variables|Default|GetSparksPS) "Sparks" _returnvalue)
  (Effects|Components|ParticleSystem|SetEmitterEnable (Variables|Default|GetSparksPS1) "Sparks" _returnvalue))

(fn ConstructionScript
  (|CallParentFunction))

(fn PlayRateChange
  (bind _returnvalue (Math|Random|RandomFloatinRange 0.1 0.5))
  (Utilities|FlowControl|Sequence
    (:then_0
      (Components|Timeline|SetPlayRate (Variables|Default|GetSkeletalMeshComponent) _returnvalue))
    (:then_1
      (Effects|Components|ParticleSystem|SetFloatParameter (Variables|Default|GetSparksPS) "SpawnRate" _returnvalue)
      (Effects|Components|ParticleSystem|SetFloatParameter (Variables|Default|GetSparksPS1) "SpawnRate" _returnvalue))))